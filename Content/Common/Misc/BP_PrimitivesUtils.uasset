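; BP_PrimitivesUtils is a small set of helper functions for reading and validating the text of an input field.
; Each helper takes the field and calls GetText on it.
; One returns the text as is, one reports whether it is empty, and one checks that its length meets a given minimum.
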(fn `CheckInputFieldContentLength`
  (params (InputField :type "/XsollaLogin/Common/Components/Interface/BPI_PrimitivesInput Interface") (MinLength :type Integer :default 1))
  (returns (IsValidLength :type Boolean))
  (bind _text (`/XsollaLogin/Common/Components/Interface/BPI_PrimitivesInput.GetText` InputField))
  (return (>= (`KismetStringLibrary.Len` _text) MinLength)))

(fn `GetTextFromInputField`
  (params (InputField :type "/XsollaLogin/Common/Components/Interface/BPI_PrimitivesInput Interface"))
  (returns (Text :type String))
  (bind _text (`/XsollaLogin/Common/Components/Interface/BPI_PrimitivesInput.GetText` InputField))
  (return _text))

(fn `IsInputFieldContentEmpty`
  (params (InputField :type "/XsollaLogin/Common/Components/Interface/BPI_PrimitivesInput Interface"))
  (returns (IsEmpty :type Boolean))
  (bind _text (`/XsollaLogin/Common/Components/Interface/BPI_PrimitivesInput.GetText` InputField))
  (return (`KismetStringLibrary.IsEmpty` _text)))