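; Login job that keeps the Xsolla OAuth 2.0 token fresh.
; It takes the expiry from the stored expiration time, or the token's "exp" claim if that is zero, and refreshes when under 30 seconds remain.
; A one-shot 30-second timer repeats the check after each pass or successful refresh, and can be cancelled.
; A failed refresh shows an error popup and schedules no further check.
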(event `self.CheckTokenExpiration`
  (bind _expiresat (`/XsollaLogin/Login/Misc/BP_TokenUtils.Get Token Expiration Time`))
  ;[1 1 1] Check token status and refresh if needed (OAuth 2.0 only)
  (bind _paramvalue (`XsollaUtilsTokenParser.GetInt64TokenParam` (`/XsollaLogin/Login/Misc/BP_TokenUtils.GetToken`) "exp"))
  (if (< (- (`XsollaUtilsLibrary.MakeDateTimeFromTimestamp` (select `bool` (!= _expiresat 0) :`false` _paramvalue :`true` _expiresat)) (`KismetMathLibrary.UtcNow`)) (`KismetMathLibrary.MakeTimespan` 0 0 0 30))
    (`XsollaLoginSubsystem.RefreshToken` (subsystem `XsollaLoginSubsystem`) (`/XsollaLogin/Login/Misc/BP_TokenUtils.GetRefreshToken`) (delegate `OnRefreshTokenSuccess`) (delegate `OnRefreshTokenError`))
    (else
      (bind _returnvalue (`KismetSystemLibrary.K2_SetTimerDelegate` (delegate `OnRepeatTokenExpirationCheck`) 30.0 :!label _label))
      (set `self.RefreshTokenJob` _returnvalue))))

(event `OnRefreshTokenSuccess`
  (params (LoginData :type "XsollaLoginData Structure (by ref)"))
  ;[1 1 1] Check token status and refresh if needed (OAuth 2.0 only)
  (goto _label))

(event `OnRefreshTokenError`
  (params (Code :type String) (Description :type String))
  ;[1 1 1] Check token status and refresh if needed (OAuth 2.0 only)
  (`/XsollaLogin/Common/BP_DemoUtils.ShowMessagePopup` (`KismetTextLibrary.Conv_StringToText` Description) true))

(event `OnRepeatTokenExpirationCheck`
  ;[1 1 1] Check token status and refresh if needed (OAuth 2.0 only)
  (`self.CheckTokenExpiration`))

(event `self.KillRefreshTokenTimer`
  (if (`KismetSystemLibrary.K2_IsValidTimerHandle` (`self.RefreshTokenJob`))
    (`KismetSystemLibrary.K2_ClearAndInvalidateTimerHandle` (`self.RefreshTokenJob`))))