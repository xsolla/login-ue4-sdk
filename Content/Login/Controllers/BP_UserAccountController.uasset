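; Controller for the user account panel in the Xsolla login demo, handling profile edits, avatar, phone number, password reset and account linking.
; Each request shows a loader, calls XsollaLoginSubsystem, then on success usually rebuilds user details data to refresh the panel or demo headers.
; Account linking takes a code from a popup, links, then re-authenticates the platform account.
; After authorization, empty nicknames get the username or, if enabled, a prompt.
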(event `self.RefreshUserAccountPanel`
  (params (Panel :type "/XsollaLogin/Login/Interface/BPI_UserAccountPanel Interface"))
  ;[1 1 1] Refresh user details
  (`/XsollaLogin/Common/BP_DemoUtils.ShowLoader` true)
  (`XsollaLoginSubsystem.UpdateUserDetails` (subsystem `XsollaLoginSubsystem`) (`/XsollaLogin/Login/Misc/BP_TokenUtils.GetToken`) (delegate `OnUserDetailsUpdateSuccess`) (`|CreateDelegate` :!event `ShowLoginError`)))

(event `OnUserDetailsUpdateSuccess`
  ;[1 1 1] Refresh user details
  (`/XsollaLogin/Common/BP_DemoUtils.ShowLoader` false)
  (bind _userdata (`self.CreateUserDetailsData`))
  (`/XsollaLogin/Login/Interface/BPI_UserAccountPanel.RefreshUserAccountDetails` (stale `self.RefreshUserAccountPanel` Panel) _userdata)
  (`/XsollaLogin/Login/Interface/BPI_UserAccountPanel.RefreshAccountLinkingStatus` (stale `self.RefreshUserAccountPanel` Panel) (not (`self.IsAccountLinkingRequired`)))
  (`/XsollaLogin/Login/Interface/BPI_DemoWidget.ActivateUserAccountPanel` (`self.DemoWidget`)))

(event `self.OnAccountLinkingInitiated`
  (params (UserAccountPanel :type "/XsollaLogin/Login/Interface/BPI_UserAccountPanel Interface") (ResultHandler :type "/XsollaLogin/Common/Handlers/BPI_ResultHandler Interface") (RefreshUserDataHandler :type "/XsollaLogin/Common/Handlers/BPI_ResultHandler Interface"))
  ;[1 1 1] link account
  (bind _returnvalue (`|CreateWidget` "/XsollaLogin/Login/Popup/W_AccountLinkingPopup.W_AccountLinkingPopup_C" (`GameplayStatics.GetPlayerController` 0)))
  (`UserWidget.AddToViewport` _returnvalue 10000)
  (add `/XsollaLogin/Login/Popup/W_AccountLinkingPopup.OnPopupResult` _returnvalue (delegate `OnAccountLinkingPopupResult`))
  (`XsollaLoginLibrary.LaunchPlatfromBrowser` (`/XsollaLogin/Common/BP_DemoUtils.GetXsollaLink` "NewEnumerator9")))

(event `OnAccountLinkingPopupResult`
  (params (IsConfirmed :type Boolean) (Code :type String))
  ;[1 1 1] link account
  (if IsConfirmed
    (`/XsollaLogin/Common/BP_DemoUtils.ShowLoader` true)
    (`XsollaLoginSubsystem.LinkAccount` (subsystem `XsollaLoginSubsystem`) (`/XsollaLogin/Login/Misc/BP_TokenUtils.GetTokenParameter` "id") (`XsollaLoginSettings.Platform` (`XsollaLoginLibrary.GetLoginSettings`)) Code (delegate `OnLinkAccountSuccess`) (`|CreateDelegate` :!event `ShowLoginError`))))

(event `OnLinkAccountSuccess`
  ;[1 1 1] link account
  (`XsollaLoginSubsystem.AuthenticatePlatformAccountUser` (subsystem `XsollaLoginSubsystem`) (`/XsollaLogin/Login/Misc/BP_TokenUtils.GetTokenParameter` "id") (`XsollaLoginSettings.Platform` (`XsollaLoginLibrary.GetLoginSettings`)) (delegate `OnPlatformAuthSucces`) (`|CreateDelegate` :!event `ShowLoginError`)))

(event `OnPlatformAuthSucces`
  (params (LoginData :type "XsollaLoginData Structure (by ref)"))
  ;[1 1 1] link account
  (`/XsollaLogin/Common/BP_DemoUtils.ShowLoader` false)
  (`self.RefreshUserData` false (stale `self.OnAccountLinkingInitiated` RefreshUserDataHandler))
  (`/Engine/EditorBlueprintResources/StandardMacros.IsValid` (`KismetSystemLibrary.Conv_InterfaceToObject` (stale `self.OnAccountLinkingInitiated` UserAccountPanel))
    (:`Is Valid`
      (`/XsollaLogin/Login/Interface/BPI_UserAccountPanel.RefreshAccountLinkingStatus` (stale `self.OnAccountLinkingInitiated` UserAccountPanel) (`/XsollaLogin/Login/Misc/BP_TokenUtils.IsMasterAccount`)))
    (:`Is Not Valid`
      _))
  (`/Engine/EditorBlueprintResources/StandardMacros.IsValid` (`KismetSystemLibrary.Conv_InterfaceToObject` (stale `self.OnAccountLinkingInitiated` ResultHandler))
    (:`Is Valid`
      (`/XsollaLogin/Common/Handlers/BPI_ResultHandler.HandleResult` (stale `self.OnAccountLinkingInitiated` ResultHandler)))))

(event `self.RefreshUserData`
  (params (bIsAfterAuthorization :type Boolean) (Handler :type "/XsollaLogin/Common/Handlers/BPI_ResultHandler Interface"))
  ;[1 1 1] refresh user data
  (if (not (`XsollaLoginSettings.bCustomAuthViaAccessToken` (`XsollaLoginLibrary.GetLoginSettings`)))
    (`/XsollaLogin/Common/BP_DemoUtils.ShowLoader` true)
    (`XsollaLoginSubsystem.UpdateUserDetails` :`self` (subsystem `XsollaLoginSubsystem`) :`AuthToken` (`/XsollaLogin/Login/Misc/BP_TokenUtils.GetToken`) :`SuccessCallback` (delegate `OnUserShortInfoUpdateSuccess`)))
  (`/Engine/EditorBlueprintResources/StandardMacros.IsValid` (`KismetSystemLibrary.Conv_InterfaceToObject` Handler)
    (:`Is Valid`
      (`/XsollaLogin/Common/Handlers/BPI_ResultHandler.HandleResult` Handler))))

(event `OnUserShortInfoUpdateSuccess`
  ;[1 1 1] refresh user data
  (`self.UpdateUserInfoInHeaders` null)
  (`self.CheckUserNickname` (stale `self.RefreshUserData` bIsAfterAuthorization))
  (`/XsollaLogin/Common/BP_DemoUtils.ShowLoader` false))

(event `self.OnLinkingCodeRequestInitiated`
  ;[1 1 1] Request account linking code
  (`/XsollaLogin/Common/BP_DemoUtils.ShowLoader` true)
  (`XsollaLoginSubsystem.CreateAccountLinkingCode` (subsystem `XsollaLoginSubsystem`) (`/XsollaLogin/Login/Misc/BP_TokenUtils.GetToken`) (delegate `OnLinkingCodeSuccess`) (`|CreateDelegate` :!event `ShowLoginError`)))

(event `OnLinkingCodeSuccess`
  (params (Code :type String))
  ;[1 1 1] Request account linking code
  (`/XsollaLogin/Common/BP_DemoUtils.ShowLoader` false)
  (`/XsollaLogin/Common/BP_DemoUtils.ShowMessagePopup` (`KismetTextLibrary.Conv_StringToText` (`KismetStringLibrary.Concat_StrStr` "YOUR CODE: " (`KismetStringLibrary.ToUpper` Code)))))

(event `self.OnSaveAvatarInitiated`
  (params (NewAvatar :type "Texture2D Object Reference") (UserAccountPanel :type "/XsollaLogin/Login/Interface/BPI_UserAccountPanel Interface"))
  ;[1 1 1] Update user avatar
  (`/XsollaLogin/Common/BP_DemoUtils.ShowLoader` true)
  (`XsollaLoginSubsystem.ModifyUserProfilePicture` (subsystem `XsollaLoginSubsystem`) (`/XsollaLogin/Login/Misc/BP_TokenUtils.GetToken`) NewAvatar (delegate `OnUserProfilePictureModificationSuccess`) (`|CreateDelegate` :!event `ShowLoginError`)))

(event `OnUserProfilePictureModificationSuccess`
  ;[1 1 1] Update user avatar
  (`/XsollaLogin/Common/BP_DemoUtils.ShowLoader` false)
  (bind _userdata (`self.CreateUserDetailsData`))
  (`/XsollaLogin/Login/Interface/BPI_UserAccountPanel.RefreshUserAccountDetails` (stale `self.OnSaveAvatarInitiated` UserAccountPanel) _userdata)
  (`/XsollaLogin/Login/Interface/BPI_UserAccountPanel.RefreshUserAvatar` (stale `self.OnSaveAvatarInitiated` UserAccountPanel) (stale `self.OnSaveAvatarInitiated` NewAvatar))
  (`self.UpdateUserInfoInHeaders` (stale `self.OnSaveAvatarInitiated` NewAvatar)))

(event `self.OnUserDetailsModificationInitiated`
  (params (Birthday :type String) (FirstName :type String) (LastName :type String) (Gender :type String) (Nickname :type String) (UserAccountPanel :type "/XsollaLogin/Login/Interface/BPI_UserAccountPanel Interface"))
  ;[1 1 1] Update user account details
  (`/XsollaLogin/Common/BP_DemoUtils.ShowLoader` true)
  (`XsollaLoginSubsystem.ModifyUserDetails` (subsystem `XsollaLoginSubsystem`) (`/XsollaLogin/Login/Misc/BP_TokenUtils.GetToken`) Birthday FirstName LastName Gender Nickname (delegate `OnUserDetailsModificationSuccess`) (`|CreateDelegate` :!event `ShowLoginError`)))

(event `OnUserDetailsModificationSuccess`
  ;[1 1 1] Update user account details
  (`/XsollaLogin/Common/BP_DemoUtils.ShowLoader` false)
  (bind _userdata (`self.CreateUserDetailsData`))
  (`/XsollaLogin/Login/Interface/BPI_UserAccountPanel.RefreshUserAccountDetails` (stale `self.OnUserDetailsModificationInitiated` UserAccountPanel) _userdata)
  (`self.UpdateUserInfoInHeaders` null))

(event `self.OnUserPhoneNumberModificationInitiated`
  (params (PhoneNumber :type String) (UserAccountPanel :type "/XsollaLogin/Login/Interface/BPI_UserAccountPanel Interface"))
  ;[1 1 1] Update user phone number
  (`/XsollaLogin/Common/BP_DemoUtils.ShowLoader` true)
  (`XsollaLoginSubsystem.ModifyUserPhoneNumber` (subsystem `XsollaLoginSubsystem`) (`/XsollaLogin/Login/Misc/BP_TokenUtils.GetToken`) PhoneNumber (delegate `OnPhoneNumberModificationSuccess`) (`|CreateDelegate` :!event `ShowLoginError`)))

(event `OnPhoneNumberModificationSuccess`
  ;[1 1 1] Update user phone number
  (`/XsollaLogin/Common/BP_DemoUtils.ShowLoader` false)
  (bind _userdata (`self.CreateUserDetailsData`))
  (`/XsollaLogin/Login/Interface/BPI_UserAccountPanel.RefreshUserAccountDetails` (stale `self.OnUserPhoneNumberModificationInitiated` UserAccountPanel) _userdata))

(event `self.OnDeleteAvatarInitiated`
  (params (UserAccountPanel :type "/XsollaLogin/Login/Interface/BPI_UserAccountPanel Interface"))
  ;[1 1 1] Remove user avatar
  (`/XsollaLogin/Common/BP_DemoUtils.ShowLoader` true)
  (`XsollaLoginSubsystem.RemoveProfilePicture` (subsystem `XsollaLoginSubsystem`) (`/XsollaLogin/Login/Misc/BP_TokenUtils.GetToken`) (delegate `OnRemoveProfilePictureSuccess`) (`|CreateDelegate` :!event `ShowLoginError`)))

(event `OnRemoveProfilePictureSuccess`
  ;[1 1 1] Remove user avatar
  (`/XsollaLogin/Common/BP_DemoUtils.ShowLoader` false)
  (bind _userdata (`self.CreateUserDetailsData`))
  (`/XsollaLogin/Login/Interface/BPI_UserAccountPanel.RefreshUserAccountDetails` (stale `self.OnDeleteAvatarInitiated` UserAccountPanel) _userdata)
  (`/XsollaLogin/Login/Interface/BPI_UserAccountPanel.RefreshUserAvatar` (stale `self.OnDeleteAvatarInitiated` UserAccountPanel) "/XsollaLogin/Common/Assets/Avatars/T_AvatarPlaceholder.T_AvatarPlaceholder")
  (`self.UpdateUserInfoInHeaders` null))

(event `self.OnPasswordResetInitiated`
  ;[1 1 1] Reset user password
  (`/XsollaLogin/Common/BP_DemoUtils.ShowLoader` true)
  (`XsollaLoginSubsystem.ResetUserPassword` (subsystem `XsollaLoginSubsystem`) (select `EUserDataStorage` (`XsollaLoginSettings.UserDataStorage` (`XsollaLoginLibrary.GetLoginSettings`)) :`Xsolla` (`/XsollaLogin/Login/Misc/BP_TokenUtils.GetTokenParameter` "username") :`Custom` (`/XsollaLogin/Login/Misc/BP_TokenUtils.GetTokenParameter` "email")) (delegate `OnPasswordResetSuccess`) (`|CreateDelegate` :!event `ShowLoginError`)))

(event `OnPasswordResetSuccess`
  ;[1 1 1] Reset user password
  (`/XsollaLogin/Common/BP_DemoUtils.ShowLoader` false)
  (bind _returnvalue (`|CreateWidget` "/XsollaLogin/Login/Popup/W_PasswordResetPopup.W_PasswordResetPopup_C" (`GameplayStatics.GetPlayerController` 0) (`/XsollaLogin/Login/Misc/BP_TokenUtils.GetTokenParameter` "email")))
  (`UserWidget.AddToViewport` _returnvalue 10000))

(event `self.OnUserPhoneNumberDeletionInitiated`
  (params (PhoneNumber :type String) (UserAccountPanel :type "/XsollaLogin/Login/Interface/BPI_UserAccountPanel Interface"))
  ;[1 1 1] Remove user phone number
  (`/XsollaLogin/Common/BP_DemoUtils.ShowLoader` true)
  (`XsollaLoginSubsystem.RemoveUserPhoneNumber` (subsystem `XsollaLoginSubsystem`) (`/XsollaLogin/Login/Misc/BP_TokenUtils.GetToken`) PhoneNumber (delegate `OnRemovePhoneNumberSuccess`) (`|CreateDelegate` :!event `ShowLoginError`)))

(event `OnRemovePhoneNumberSuccess`
  ;[1 1 1] Remove user phone number
  (`/XsollaLogin/Common/BP_DemoUtils.ShowLoader` false)
  (bind _userdata (`self.CreateUserDetailsData`))
  (`/XsollaLogin/Login/Interface/BPI_UserAccountPanel.RefreshUserAccountDetails` (stale `self.OnUserPhoneNumberDeletionInitiated` UserAccountPanel) _userdata))

(fn `CheckUserNickname`
  (params (bIsAfterAuthorization :type Boolean))
  (if bIsAfterAuthorization
    (if (`KismetStringLibrary.EqualEqual_StrStr` (`/XsollaLogin/Login/Misc/BP_TokenUtils.GetTokenParameter` "type") "xsolla_login")
      (if (`self.IsNicknameSet`)
        (`self.UpdateUserNickname` (`/XsollaLogin/Login/Misc/BP_TokenUtils.GetTokenParameter` "username")))
      (elif (and (`self.IsNicknameSet`) (`XsollaLoginSettings.RequestNickname` (`XsollaLoginLibrary.GetLoginSettings`)))
        (bind _returnvalue (`|CreateWidget` "/XsollaLogin/Login/Popup/W_NicknamePopup.W_NicknamePopup_C" (`GameplayStatics.GetPlayerController` 0)))
        (`UserWidget.AddToViewport` _returnvalue 10000)
        (add `/XsollaLogin/Login/Popup/W_NicknamePopup.OnPopupResult` _returnvalue (`|CreateDelegate` :!event `HandleNicknamePopupResult`))))))

(fn `CreateHeaderData`
  (params (Avatar :type "Texture2D Object Reference"))
  (returns (UserData :type "/XsollaLogin/Common/Interface/BPI_HeaderData Interface"))
  (bind (_ban _birthday _connection_information _country _email _external_id _first_name _gender _groups _id _is_anonymous _last_login _last_name _name _nickname _tag _phone _picture) (break `XsollaUserDetails` (`XsollaLoginSubsystem.GetUserDetails` (subsystem `XsollaLoginSubsystem`))))
  (bind _returnvalue (`|GenericCreateObject` "/XsollaLogin/Common/Data/BP_HeaderData.BP_HeaderData_C" (`GameplayStatics.GetPlayerController` 0) (select `bool` (`KismetSystemLibrary.IsValid` Avatar) :`true` (`WidgetBlueprintLibrary.MakeBrushFromTexture` Avatar 360 360)) (select `bool` (> (`KismetStringLibrary.Len` _nickname) 0) :`false` (select `bool` (> (`KismetStringLibrary.Len` _email) 0) :`true` _email) :`true` _nickname) _picture))
  (bind _iconsloader (`/XsollaLogin/Login/Interface/BPI_Demo.GetIconsLoader` (`self.Demo`)))
  (`/XsollaLogin/Login/Interface/BPI_IconsLoader.LoadIcons` _iconsloader (`|MakeArray` _returnvalue :!type "/XsollaLogin/Common/Interface/BPI_IconPresenter Interface"))
  (return _returnvalue))

(fn `CreateUserDetailsData`
  (returns (UserData :type "/XsollaLogin/Login/Interface/BPI_UserDetailsData Interface"))
  (bind _returnvalue (`|GenericCreateObject` "/XsollaLogin/Login/Data/BP_UserDetailsData.BP_UserDetailsData_C" self (`XsollaLoginSubsystem.GetUserDetails` (subsystem `XsollaLoginSubsystem`)) (`self.GetCurrentUserLevel`) (`/XsollaLogin/Login/Misc/BP_TokenUtils.GetTokenParameter` "username") (`KismetStringLibrary.EqualEqual_StrStr` (`/XsollaLogin/Login/Misc/BP_TokenUtils.GetTokenParameter` "type") "xsolla_login")))
  (bind _iconsloader (`/XsollaLogin/Login/Interface/BPI_Demo.GetIconsLoader` (`self.Demo`)))
  (`/XsollaLogin/Login/Interface/BPI_IconsLoader.LoadIcons` _iconsloader (`|MakeArray` _returnvalue :!type "/XsollaLogin/Common/Interface/BPI_IconPresenter Interface"))
  (return _returnvalue))

(fn `GetCurrentUserLevel`
  (returns (Value :type Integer))
  (bind _returnvalue (`GameplayStatics.LoadGameFromSlot` "UserLevelData"))
  (bind _asbp_user_level_save_data (cast `/XsollaLogin/Login/Data/BP_UserLevelSaveData` _returnvalue)
    (:`then`
      (bind (_value _returnvalue_2) (`BlueprintMapLibrary.Map_Find` (`/XsollaLogin/Login/Data/BP_UserLevelSaveData.UserLevels` _asbp_user_level_save_data) (`/XsollaLogin/Login/Misc/BP_TokenUtils.GetTokenParameter` "sub")))
      (if _returnvalue_2
        (return _value)
        (else
          (return 1))))
    (:`CastFailed`
      (return 1))))

(fn `HandleNicknamePopupResult`
  (params (IsConfirmed :type Boolean) (Nickname :type String))
  (if IsConfirmed
    (`self.UpdateUserNickname` Nickname)))

(fn `HandleNicknameSuccessfulUpdate`
  (`self.UpdateUserInfoInHeaders` null))

(fn `Init`
  (params (Demo :type "/XsollaLogin/Login/Interface/BPI_Demo Interface") (DemoWidget :type "/XsollaLogin/Login/Interface/BPI_DemoWidget Interface"))
  (set `self.Demo` Demo)
  (set `self.DemoWidget` DemoWidget))

(fn `IsAccountLinkingRequired`
  (returns (IsLinkingRequired :type Boolean))
  (bind _returnvalue (`XsollaLoginLibrary.GetLoginSettings`))
  (bind _asxsolla_demo_game_mode_base (cast `/XsollaLogin/Common/XsollaDemoGameModeBase` (`GameplayStatics.GetGameMode`)))
  (return (and (`KismetSystemLibrary.IsValidClass` (`XsollaDemoGameModeBase.GetStoreDemo` _asxsolla_demo_game_mode_base)) (`XsollaLoginSettings.UseCrossPlatformAccountLinking` _returnvalue) (`|EnumInequality` (`XsollaLoginSettings.Platform` _returnvalue) "xsolla") (not (`/XsollaLogin/Login/Misc/BP_TokenUtils.IsMasterAccount`)))))

(fn `IsNicknameSet`
  (returns (ReturnValue :type Boolean))
  (return (== (`KismetStringLibrary.Len` (`.nickname` (break `XsollaUserDetails` (`XsollaLoginSubsystem.GetUserDetails` (subsystem `XsollaLoginSubsystem`))))) 0)))

(fn `ShowLoginError`
  (params (code :type String) (description :type String))
  (`/XsollaLogin/Common/BP_DemoUtils.ShowLoginError` code description))

(fn `UpdateUserInfoInHeaders`
  (params (Avatar :type "Texture2D Object Reference"))
  (bind _userdata (`self.CreateHeaderData` Avatar))
  (`/XsollaLogin/Login/Interface/BPI_DemoWidget.RefreshHeaders` (`self.DemoWidget`) _userdata))

(fn `UpdateUserNickname`
  (params (InputPin :type String))
  (bind (_ban _birthday _connection_information _country _email _external_id _first_name _gender _groups _id _is_anonymous _last_login _last_name) (break `XsollaUserDetails` (`XsollaLoginSubsystem.GetUserDetails` (subsystem `XsollaLoginSubsystem`))))
  (`XsollaLoginSubsystem.ModifyUserDetails` :`self` (subsystem `XsollaLoginSubsystem`) :`AuthToken` (`/XsollaLogin/Login/Misc/BP_TokenUtils.GetToken`) :`FirstName` _first_name :`LastName` _last_name :`Nickname` InputPin :`SuccessCallback` (`|CreateDelegate` :!event `HandleNicknameSuccessfulUpdate`)))