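; BP_UserDetailsData is a data holder for a user's profile in the Login system.
; Getters expose fields from a UserDetails struct, such as name, contact info and picture URL, plus separate Username, Level and password-reset values.
; RefreshIcon stores a received icon as the avatar and flags it ready.
; GetAvatar returns that icon only when a picture URL exists, otherwise a blank default brush.
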(event `/XsollaLogin/Common/Interface/BPI_IconPresenter.RefreshIcon`
  (params (Icon :type "SlateBrush Structure"))
  (set `self.Avatar` Icon)
  (set `self.IsAvatarReady` true))

(fn `GetAvatar`
  (returns (Avatar :type "SlateBrush Structure"))
  (return (select `bool` (> (`KismetStringLibrary.Len` (`.picture` (break `XsollaUserDetails` (`self.UserDetails`)))) 0) :`false` (make `SlateBrush` (360.0 360.0) (struct) (struct :`SpecifiedColor` (struct :`R` 1.0 :`G` 1.0 :`B` 1.0 :`A` 1.0) :`ColorUseRule` "UseColor_Specified") "/XsollaLogin/Common/Assets/Avatars/T_AvatarPlaceholder.T_AvatarPlaceholder") :`true` (`self.Avatar`))))

(fn `GetBirthday`
  (returns (Birthday :type String))
  (return (`.birthday` (break `XsollaUserDetails` (`self.UserDetails`)))))

(fn `GetEmail`
  (returns (Email :type String))
  (return (`.email` (break `XsollaUserDetails` (`self.UserDetails`)))))

(fn `GetFirstName`
  (returns (FirstName :type String))
  (return (`.first_name` (break `XsollaUserDetails` (`self.UserDetails`)))))

(fn `GetImageUrl`
  (returns (ImageUrl :type String))
  (return (`.picture` (break `XsollaUserDetails` (`self.UserDetails`)))))

(fn `GetLastName`
  (returns (LastName :type String))
  (return (`.last_name` (break `XsollaUserDetails` (`self.UserDetails`)))))

(fn `GetLevel`
  (returns (Level :type Integer))
  (return (`self.Level`)))

(fn `GetNickname`
  (returns (Nickname :type String))
  (return (`.nickname` (break `XsollaUserDetails` (`self.UserDetails`)))))

(fn `GetPhoneNumber`
  (returns (PhoneNumber :type String))
  (return (`.phone` (break `XsollaUserDetails` (`self.UserDetails`)))))

(fn `GetTag`
  (returns (Tag :type String))
  (return (`.tag` (break `XsollaUserDetails` (`self.UserDetails`)))))

(fn `GetUserGender`
  (returns (Gender :type String))
  (return (`.gender` (break `XsollaUserDetails` (`self.UserDetails`)))))

(fn `GetUsername`
  (returns (Username :type String))
  (return (`self.Username`)))

(fn `IsIconSet`
  (returns (IsIconSet :type Boolean))
  (return (`self.IsAvatarReady`)))

(fn `IsPasswordResetAllowed`
  (returns (IsAllowed :type Boolean))
  (return (`self.PasswordResetAllowed`)))