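; Utility functions for UI Builder that apply theme colors, fonts and brushes to widgets.
; GetColor and GetFont look up a theme entry by type and fall back to a supplied default.
; The button and input field updaters rebuild widget styles from theme brushes, retaining properties such as padding, and do nothing without a valid theme.
; Input fields also use both getters for font and text color, with font size passed separately.
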(fn `GetColor`
  (params (Theme :type "XsollaUIBuilderTheme Class Reference") (ColorType :type "EColorType Enum" :default "ColorType_Default") (DefaultColor :type "SlateColor Structure"))
  (returns (Color :type "SlateColor Structure"))
  (bind _returnvalue (`XsollaUIBuilderLibrary.GetTheme` Theme))
  (bind (_bisfound _returnvalue_2) (`XsollaUIBuilderTheme.GetColorByType` _returnvalue ColorType))
  (if (and (`KismetSystemLibrary.IsValid` _returnvalue) _bisfound)
    (return (make `SlateColor` (`KismetMathLibrary.Conv_ColorToLinearColor` _returnvalue_2)))
    (else
      (return DefaultColor))))

(fn `GetFont`
  (params (Theme :type "XsollaUIBuilderTheme Class Reference") (FontType :type "EFontType Enum" :default "FontType_Default") (DefaultFont :type "SlateFontInfo Structure"))
  (returns (ReturnValue :type "SlateFontInfo Structure (by ref)"))
  (bind _returnvalue (`XsollaUIBuilderLibrary.GetTheme` Theme))
  (bind (_bisfound _returnvalue_2) (`XsollaUIBuilderTheme.GetFontByType` _returnvalue FontType))
  (if (and (`KismetSystemLibrary.IsValid` _returnvalue) _bisfound)
    (return _returnvalue_2)
    (else
      (return DefaultFont))))

(fn `UpdateButtonThemeStyle`
  (params (Theme :type "XsollaUIBuilderTheme Class Reference") (NormalStateType :type "EBrushThemeType Enum" :default "BrushType_Default") (HoverStateType :type "EBrushThemeType Enum" :default "BrushType_Default") (PressedStateType :type "EBrushThemeType Enum" :default "BrushType_Default") (DisabledStateType :type "EBrushThemeType Enum" :default "BrushType_Default") (Button :type "Button Object Reference"))
  (bind _returnvalue (`XsollaUIBuilderLibrary.GetTheme` Theme))
  (bind (_normal _hovered _pressed _disabled _normalpadding _pressedpadding _pressedslatesound _hoveredslatesound) (break `ButtonStyle` (`Button.WidgetStyle` Button)))
  (`/Engine/EditorBlueprintResources/StandardMacros.IsValid` _returnvalue
    (:`Is Valid`
      (`Button.SetStyle` Button (make `ButtonStyle` (`.ReturnValue` (`XsollaUIBuilderTheme.GetBrushByType` _returnvalue NormalStateType)) (`.ReturnValue` (`XsollaUIBuilderTheme.GetBrushByType` _returnvalue HoverStateType)) (`.ReturnValue` (`XsollaUIBuilderTheme.GetBrushByType` _returnvalue PressedStateType)) (`.ReturnValue` (`XsollaUIBuilderTheme.GetBrushByType` _returnvalue DisabledStateType)) _normalpadding _pressedpadding _pressedslatesound _hoveredslatesound)))))

(fn `UpdateInputFieldThemeStyle`
  (params (Theme :type "XsollaUIBuilderTheme Class Reference") (NormalStateBrush :type "EBrushThemeType Enum" :default "BrushType_Default") (HoverStateBrush :type "EBrushThemeType Enum" :default "BrushType_Default") (ActiveStateBrush :type "EBrushThemeType Enum" :default "BrushType_Default") (DisabledStateBrush :type "EBrushThemeType Enum" :default "BrushType_Default") (FontType :type "EFontType Enum" :default "FontType_Default") (FontSize :type Integer) (TextColor :type "EColorType Enum" :default "ColorType_Default") (InputField :type "EditableTextBox Object Reference"))
  (bind _returnvalue (`XsollaUIBuilderLibrary.GetTheme` Theme))
  (bind (_backgroundimagenormal _backgroundimagehovered _backgroundimagefocused _backgroundimagereadonly _padding _font _foregroundcolor _backgroundcolor _readonlyforegroundcolor _hscrollbarpadding _vscrollbarpadding _scrollbarstyle) (break `EditableTextBoxStyle` (`EditableTextBox.WidgetStyle` InputField)))
  (bind (_fontobject _fontmaterial _outlinesettings _typefacefontname _size _letterspacing) (break `SlateFontInfo` (`self.GetFont` Theme FontType (make `SlateFontInfo` "/XsollaLogin/Common/Assets/Font/Font_Roboto-Regular.Font_Roboto-Regular" null (struct :`OutlineColor` (struct :`A` 1.0)) "None" 14))))
  (`/Engine/EditorBlueprintResources/StandardMacros.IsValid` _returnvalue
    (:`Is Valid`
      (set `EditableTextBox.WidgetStyle` (make `EditableTextBoxStyle` (`.ReturnValue` (`XsollaUIBuilderTheme.GetBrushByType` _returnvalue NormalStateBrush)) (`.ReturnValue` (`XsollaUIBuilderTheme.GetBrushByType` _returnvalue HoverStateBrush)) (`.ReturnValue` (`XsollaUIBuilderTheme.GetBrushByType` _returnvalue ActiveStateBrush)) (`.ReturnValue` (`XsollaUIBuilderTheme.GetBrushByType` _returnvalue DisabledStateBrush)) _padding (make `SlateFontInfo` _fontobject _fontmaterial _outlinesettings _typefacefontname FontSize _letterspacing) (`self.GetColor` Theme TextColor (make `SlateColor` (struct :`R` 1.0 :`G` 1.0 :`B` 1.0 :`A` 0.7))) _backgroundcolor _readonlyforegroundcolor _hscrollbarpadding _vscrollbarpadding _scrollbarstyle) InputField))))